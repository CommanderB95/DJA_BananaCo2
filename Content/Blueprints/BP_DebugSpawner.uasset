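; BP_DebugSpawner is a debug actor that wraps a BP_Spawner child actor and spawns a dummy when F is pressed.
; The construction script passes its FirstWaypoint and Objective to the child spawner, and BeginPlay sets that spawner inactive and prints a hello message.
; Collision begin and end overlaps toggle input and a component's visibility, with no check on which actor overlaps.
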(event `self.ReceiveBeginPlay`
  (bind _asbp_spawner (cast `/Game/Blueprints/BP_Spawner` (`ChildActorComponent.ChildActor` (`self.Spawner`))))
  (set `/Game/Blueprints/BP_Spawner.IsActive` false _asbp_spawner)
  (`KismetSystemLibrary.PrintString` "Hello"))

(event `self.ReceiveActorBeginOverlap`
  (params (OtherActor :type "Actor Object Reference")))

(event `self.ReceiveTick`
  (params (DeltaSeconds :type "Float (single-precision)")))

(event `self.CollisionComponent.OnComponentBeginOverlap`
  (params (OtherActor :type "Actor Object Reference") (OtherComp :type "PrimitiveComponent Object Reference") (OtherBodyIndex :type Integer) (bFromSweep :type Boolean) (SweepResult :type "EngineTypes.HitResult Structure (by ref)"))
  (`self.EnableInput` (`GameplayStatics.GetPlayerController` 0))
  (`SceneComponent.SetVisibility` true))

(event `self.CollisionComponent.OnComponentEndOverlap`
  (params (OtherActor :type "Actor Object Reference") (OtherComp :type "PrimitiveComponent Object Reference") (OtherBodyIndex :type Integer))
  (`self.DisableInput` (`GameplayStatics.GetPlayerController` 0) null)
  (`SceneComponent.SetVisibility` false))

(event `Key|F`
  (:`Pressed`
    (bind _asbp_spawner (cast `/Game/Blueprints/BP_Spawner` (`ChildActorComponent.ChildActor` (`self.Spawner`))))
    (`/Game/Blueprints/BP_Spawner.SpawnDummy` _asbp_spawner)))

(fn `UserConstructionScript`
  (bind _asbp_spawner (cast `/Game/Blueprints/BP_Spawner` (`ChildActorComponent.ChildActor` (`self.Spawner`))))
  (set `/Game/Blueprints/BP_Spawner.FirstWaypoint` (`self.FirstWaypoint`) _asbp_spawner)
  (set `/Game/Blueprints/BP_Spawner.Objective` (`self.Objective`) _asbp_spawner))