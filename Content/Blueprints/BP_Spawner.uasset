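; BP_Spawner is a spawner actor that periodically creates groups of BP_Dummy AI pawns around its location.
; While IsActive is set, Tick accumulates time and calls SpawnDummy at a fixed interval.
; SpawnDummy spawns a randomly sized batch at random points within a radius, each with the BehaviorTree variable's tree.
; It then assigns FirstWaypoint to each dummy's BP_AIController as its Waypoint.
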(event `self.ReceiveBeginPlay`)

(event `self.ReceiveActorBeginOverlap`
  (params (OtherActor :type "Actor Object Reference")))

(event `self.ReceiveTick`
  (params (DeltaSeconds :type "Float (single-precision)"))
  (if (`self.IsActive`)
    (bind _output_get (set `self.DeltaTime` (+ DeltaSeconds (`self.DeltaTime`))))
    (if (>= _output_get 5.0)
      (`self.SpawnDummy`)
      (set `self.DeltaTime` 0.0))))

(event `SpawnDummy`
  (for _ (range (+ (`KismetMathLibrary.RandomIntegerInRange` 2 7) 1))
    (bind _returnvalue (`AIBlueprintHelperLibrary.SpawnAIFromClass` "/Game/AI/BP_Dummy.BP_Dummy_C" "/Game/AI/BehaviorTree.BehaviorTree" (`NavigationSystem.GetRandomPointInRadius` (`self.K2_GetActorLocation`) 500.0)))
    (bind _asbp_dummy (cast `/Game/AI/BP_Dummy` _returnvalue))
    (bind _returnvalue_2 (`AIBlueprintHelperLibrary.GetAIController` _asbp_dummy))
    (bind _asbp_aicontroller (cast `/Game/AI/BP_AIController` _returnvalue_2))
    (set `/Game/AI/BP_AIController.Waypoint` (`self.FirstWaypoint`) _asbp_aicontroller)))

(fn `UserConstructionScript`)