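; BP_Dummy is a damageable AI dummy that remembers its attacking player and alerts nearby dummies.
; Point damage lowers Health and stores a BP_Player causer as TargetRef; non-fatal hits sphere-trace for pawns, passing TargetRef to dummies found and setting their IsTargetBox flag.
; Health at exactly zero plays a death animation, clears IsAlive and removes the capsule.
; Tick destroys the dead actor after ten seconds.
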(event `self.ReceiveTick`
  (params (DeltaSeconds :type "Float (single-precision)"))
  ;[1 1 1] Destroy Actor after 10 seconds.
  (if (not (`self.IsAlive`))
    (bind _output_get (set `self.DeltaTime` (+ DeltaSeconds (`self.DeltaTime`))))
    (if (>= _output_get 10.0)
      (`self.K2_DestroyActor`))))

(event `self.ReceivePointDamage`
  (params (Damage :type "Float (single-precision)") (DamageType :type "DamageType Object Reference") (HitLocation :type "Object.Vector Structure") (HitNormal :type "Object.Vector Structure") (HitComponent :type "PrimitiveComponent Object Reference") (BoneName :type Name) (ShotFromDirection :type "Object.Vector Structure") (InstigatedBy :type "Controller Object Reference") (DamageCauser :type "Actor Object Reference"))
  (bind _returnvalue (`self.K2_GetActorLocation`))
  (bind _asbp_player (cast `/Game/Blueprints/BP_Player` DamageCauser)
    (:`then`
      (set `self.Target_Ref` _asbp_player))
    (:`CastFailed`
      _))
  ;[1 1 1] Apply Damage to Health
  (bind _output_get (set `self.Health` (- (`self.Health`) Damage)))
  (if (== _output_get 0.0)
    (`SkeletalMeshComponent.PlayAnimation` (`self.Mesh`) "/Game/AnimStarterPack/Death_1.Death_1" false)
    (set `self.IsAlive` false)
    (`ActorComponent.K2_DestroyComponent` (`self.CapsuleComponent`))
    (else
      (set `self.IsTargetBox` false)
      (bind (_outhits _returnvalue_2) (`KismetSystemLibrary.SphereTraceMultiForObjects` :`Start` _returnvalue :`End` (+ _returnvalue (0.0 0.0 15.0)) :`Radius` 1000.0 :`ObjectTypes` (`|MakeArray` "ObjectTypeQuery3" :!type "EngineTypes.EObjectTypeQuery Enum") :`DrawDebugType` "ForDuration" :`bIgnoreSelf` false))
      (for _array_element _outhits
        (bind _asbp_dummy (cast `/Game/AI/BP_Dummy` (`.HitActor` (`GameplayStatics.BreakHitResult` _array_element))))
        (set `/Game/AI/BP_Dummy.Target_Ref` (`self.Target_Ref`) _asbp_dummy)
        (set `/Game/AI/BP_Dummy.IsTargetBox` true _asbp_dummy)))))

(fn `UserConstructionScript`)